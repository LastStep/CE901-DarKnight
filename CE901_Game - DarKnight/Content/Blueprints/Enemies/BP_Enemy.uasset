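; BP_Enemy is an enemy character whose health, speed, gravity, attack hitbox and drops are driven by EnemyData.
; Attack events set combat state and animation; on finish, melee damages characters overlapping the box, while ranged damages the player if a visibility trace is unblocked.
; Hits subtract ability damage, update health text and play a damage animation.
; Death updates the game mode's enemy count, spawns a type-specific drop and destroys the actor.
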(event `self.ReceiveBeginPlay`
  (`self.SetParameters`))

(event `/Game/Blueprints/Interface/BPI_Hit.onTakingDamage`
  (params (Enemy :type "/Game/Blueprints/Enemies/BP_Enemy Object Reference") (`Damage Ability` :type "/Game/Blueprints/GameplayAbilities/BP_GameplayAbility Object Reference"))
  (`self.OnHit` `Damage Ability`))

(event `EventOnDeath`
  (`KismetSystemLibrary.Delay` 0.5)
  (`ActorComponent.K2_DestroyComponent` (`self.UIHealth`))
  (`self.K2_DestroyActor`))

(event `Event On Attacking`
  (`self.OnAttacking`))

(event `EventOnAttackFinish`
  (`self.DispatchOnAttackEnd`)
  (`self.OnAttackFinish`))

(fn `CheckDeath`
  (returns (isDead :type Boolean))
  (bind _output_get (set `self.isAlive` (> (`self.Health`) 0)))
  (return (not _output_get)))

(fn `Get Ideal Range`
  (returns (`Attack Radius` :type "Float (double-precision)") (`Defend Radius` :type "Float (double-precision)"))
  (return 10.0 20.0))

(fn `OnAttackFinish`
  (switch `/Game/Data/Enemy/E_EnemyAttackType` (`/Game/Data/Enemy/BP_EnemyDataAsset.AttackType` (`self.EnemyData`))
    (:`NewEnumerator0`
      (for _array_element (`PrimitiveComponent.GetOverlappingActors` (`self.AttackHitBox`) "/Game/Blueprints/Heroes/PaperZD/BP_Character.BP_Character_C")
        (bind _asbp_character (cast `/Game/Blueprints/Heroes/PaperZD/BP_Character` _array_element))
        (`/Game/Blueprints/Heroes/PaperZD/BP_Character.On Hit` _asbp_character null (`/Game/Data/Enemy/BP_EnemyDataAsset.BaseAttackDamage` (`self.EnemyData`)))
        (set `self.State` "NewEnumerator0")))
    (:`NewEnumerator1`
      (bind _asbp_character_2 (cast `/Game/Blueprints/Heroes/PaperZD/BP_Character` (`GameplayStatics.GetPlayerCharacter` 0)))
      (bind (_outhit _returnvalue) (`KismetSystemLibrary.LineTraceSingle` :`Start` (`self.K2_GetActorLocation`) :`End` (`self.K2_GetActorLocation` _asbp_character_2) :`TraceChannel` "TraceTypeQuery1" :`TraceColor` (struct :`R` 0.784722 :`G` 0.100815 :`B` 0.100815 :`A` 1.0) :`TraceHitColor` (struct :`G` 1.0) :`DrawTime` 0.3))
      (if (not _returnvalue)
        (`/Game/Blueprints/Heroes/PaperZD/BP_Character.On Hit` _asbp_character_2 self (`/Game/Data/Enemy/BP_EnemyDataAsset.BaseAttackDamage` (`self.EnemyData`))))
      (set `self.State` "NewEnumerator0"))))

(fn `OnAttacking`
  (switch `/Game/Data/Enemy/E_EnemyState` (`self.State`)
    (:`NewEnumerator0`
      _)
    (:`NewEnumerator1`
      _)
    (:`NewEnumerator2`
      _))
  (set `self.State` "NewEnumerator2")
  (`PaperZDAnimInstance.JumpToNode` (`PaperZDAnimationComponent.AnimInstance` (`self.AnimationComponent`)) "CombatStart" "Locomotion"))

(fn `OnDeath`
  (bind _asbp_play_game_mode (cast `/Game/Blueprints/Game/BP_PlayGameMode` (`GameplayStatics.GetGameMode`)))
  (`/Game/Blueprints/Game/BP_PlayGameMode.UpdateEnemyCount` _asbp_play_game_mode)
  (switch `/Game/Data/Enemy/E_Enemy` (`/Game/Data/Enemy/BP_EnemyDataAsset.Enemy` (`self.EnemyData`))
    (:`NewEnumerator2`
      (`|SpawnActorFromClass` "/Game/Blueprints/BP_EnemyDrop.BP_EnemyDrop_C" (`self.GetTransform` self) "Undefined" "MultiplyWithRoot" null (make `/Game/Data/Gameplay/ST_ItemData` 30.0) "/Game/Assets/Items/Drops/FB_DropGreen.FB_DropGreen" null :!label _label))
    (:`NewEnumerator1`
      (goto _label))
    (:`NewEnumerator3`
      (`|SpawnActorFromClass` "/Game/Blueprints/BP_EnemyDrop.BP_EnemyDrop_C" (`self.GetTransform` self) "Undefined" "MultiplyWithRoot" null (make `/Game/Data/Gameplay/ST_ItemData` 50.0) "/Game/Assets/Items/Drops/FB_DropPurple.FB_DropPurple" null)))
  (`self.EventOnDeath`))

(fn `OnHit`
  (params (`Damage Ability` :type "/Game/Blueprints/GameplayAbilities/BP_GameplayAbility Object Reference"))
  (set `self.State` "NewEnumerator3")
  (set `self.Health` (- (`self.Health`) (`/Game/Blueprints/GameplayAbilities/BP_GameplayAbility.GetDamageFromAbility` `Damage Ability`)))
  (`self.SetHealthText`)
  (bind _isdead (`self.CheckDeath`))
  (`PaperZDAnimInstance.JumpToNode` (`PaperZDAnimationComponent.AnimInstance` (`self.AnimationComponent`)) "Damaged" "Locomotion")
  (if _isdead
    (`self.OnDeath`)))

(fn `SetHealthText`
  (`TextRenderComponent.K2_SetText` (`self.UIHealth`) (`KismetTextLibrary.Conv_IntToText` (`self.Health`))))

(fn `SetParameters`
  (bind _enemydata (`self.EnemyData`))
  (set `self.isAlive` true)
  (set `self.Health` (`/Game/Data/Enemy/BP_EnemyDataAsset.MaxHealth` _enemydata))
  (set `CharacterMovementComponent.MaxWalkSpeed` (`/Game/Data/Enemy/BP_EnemyDataAsset.MaxSpeed` _enemydata) (`self.CharacterMovement`))
  (`self.SetHealthText`)
  (set `self.State` "NewEnumerator0")
  (switch `/Game/Data/Enemy/E_EnemyType` (`/Game/Data/Enemy/BP_EnemyDataAsset.EnemyType` _enemydata)
    (:`NewEnumerator3`
      (set `CharacterMovementComponent.GravityScale` 0.0 (`self.CharacterMovement`)))))

(fn `UserConstructionScript`
  (bind _attackhitbox (`self.AttackHitBox`))
  (bind _attackrange (`/Game/Data/Enemy/BP_EnemyDataAsset.AttackRange` (`self.EnemyData`)))
  (`BoxComponent.SetBoxExtent` _attackhitbox (`KismetMathLibrary.MakeVector` _attackrange 32.0 32.0) true)
  (`SceneComponent.K2_AddLocalOffset` _attackhitbox (`KismetMathLibrary.MakeVector` (/ _attackrange 2.0)) false false))