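; Play game mode that runs a 2D tile-map level for the selected playtest, hero and level.
; On BeginPlay, Play Test 2 mirrors the layout by swapping in mirrored tile maps, starting the player on the right and flipping enemy X positions.
; Tick tracks time and kills, detecting a cleared level or player death, then pauses, shows the matching screen and saves results through BP_GameInstance.
; It also holds hero-state flag setters.
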(event `self.ReceiveBeginPlay`
  (bind _as_bp_game_instance (`self.As BP Game Instance`))
  (bind _asbp_game_instance (cast `/Game/Blueprints/Game/BP_GameInstance` (`GameplayStatics.GetGameInstance`)))
  (set `self.As BP Game Instance` _asbp_game_instance)
  (`self.SetTileMap`
    (:`Out`
      (`self.SetPlayerStart`
        (:`Out`
          (`self.FlipEnemySpawns`
            (:`Out`
              (bind _output_get (set `self.CurrentLevelData` (make `/Game/Blueprints/SaveGame/ST_LevelData` (`/Game/Blueprints/Game/BP_GameInstance.SelectedPlayTest` _as_bp_game_instance) (`/Game/Blueprints/Game/BP_GameInstance.SelectedHero` _as_bp_game_instance) (`/Game/Blueprints/Game/BP_GameInstance.SelectedLevel` _as_bp_game_instance))))
              (`KismetSystemLibrary.PrintString` (`|GetEnumeratorNameAsString` (`.Level_18_E6D6E14D441597B8F601448B6307EB99` (break `/Game/Blueprints/SaveGame/ST_LevelData` _output_get)))))))))))

(event `self.ReceiveTick`
  (params (DeltaSeconds :type "Float (single-precision)"))
  (`self.OnGameTick`
    (:`Out`
      (`self.CheckGameOver`
        (:`Yes`
          (`self.OnGameOver`))
        (:`No`
          (if (`/Game/Blueprints/Heroes/PaperZD/BP_Character.CheckDeath` (`self.As BP Character`))
            (`/Game/Blueprints/Heroes/PaperZD/BP_Character.OnPlayerDeath` (`self.As BP Character`))
            (`self.OnPlayerDeathh`)))))))

(event `/Game/Blueprints/Interface/BPI_PlayerEvents.OnPlayerDeath`)

(event `EventOnBackToMainMenu`
  (bind _gameoverwidget (`self.GameOverWidget`))
  (`/Engine/EditorBlueprintResources/StandardMacros.IsValid` _gameoverwidget
    (:`Is Valid`
      (`Widget.RemoveFromParent` _gameoverwidget))
    (:`Is Not Valid`
      _))
  (`GameplayStatics.OpenLevelBySoftObjectPtr` "/Game/Maps/Title/TitleLevel.TitleLevel"))

(fn `FlipTileMap`
  (locals (TempTileAtMirroredXY :type "PaperTileInfo Structure") (X :type Integer) (Y :type Integer) (MirroredX :type Integer) (MirroredY :type Integer) (MapWidth :type Integer :default 0) (MapHeight :type Integer :default 0) (CurrentLayer :type Integer :default 1) (MapLayers :type Integer :default 0))
  (bind (_mapwidth _mapheight _numlayers) (`PaperTileMapComponent.GetMapSize` (`PaperTileMapActor.RenderComponent` (`self.TileMap`))))
  (set `local.MapWidth` _mapwidth)
  (set `local.MapHeight` _mapheight)
  (set `local.MapLayers` _numlayers)
  (for _index (range (`local.MapLayers`))
    (set `local.CurrentLayer` _index)
    (set `local.CurrentLayer` 1)
    (for _index_2 (range (`local.MapWidth`))
      (set `local.X` _index_2)
      (for _index_3 (range (`local.MapHeight`))
        (set `local.Y` _index_3)
        (set `local.MirroredX` (- (`local.MapWidth`) 1 (`local.X`)))
        (set `local.MirroredY` (- (`local.MapHeight`) 1 (`local.Y`)))
        (set `local.TempTileAtMirroredXY` (`PaperTileMapComponent.GetTile` (`PaperTileMapActor.RenderComponent` (`self.TileMap`)) (`local.MirroredX`) (`local.MirroredY`) (`local.CurrentLayer`)))
        (`PaperTileMapComponent.SetTile` (`PaperTileMapActor.RenderComponent` (`self.TileMap`)) (`local.MirroredX`) (`local.MirroredY`) (`local.CurrentLayer`) (`PaperTileMapComponent.GetTile` (`PaperTileMapActor.RenderComponent` (`self.TileMap`)) (`local.X`) (`local.Y`) (`local.CurrentLayer`)))
        (`PaperTileMapComponent.SetTile` (`PaperTileMapActor.RenderComponent` (`self.TileMap`)) (`local.X`) (`local.Y`) (`local.CurrentLayer`) (`local.TempTileAtMirroredXY`))))))

(fn `GetCurrentLevelTime`
  (returns (`Current Level Data Time Taken` :type "Float (double-precision)"))
  (bind (_currentleveldata_playtest _currentleveldata_hero _currentleveldata_level _currentleveldata_success _currentleveldata_timetaken) (break `/Game/Blueprints/SaveGame/ST_LevelData` (`self.CurrentLevelData`)))
  (return _currentleveldata_timetaken))

(fn `OnGameOver`
  (bind _returnvalue (`GameplayStatics.GetPlayerController` 0))
  (bind (_currentleveldata_playtest _currentleveldata_hero _currentleveldata_level _currentleveldata_success _currentleveldata_timetaken _currentleveldata_enemieskilled) (break `/Game/Blueprints/SaveGame/ST_LevelData` (`self.CurrentLevelData`)))
  (bind _returnvalue_2 (`|CreateWidget` (`self.GameOverScreenWidget`)))
  (bind _output_get (set `self.GameOverWidget` _returnvalue_2))
  (`UserWidget.AddToViewport` _output_get 0)
  (set `PlayerController.bShowMouseCursor` true _returnvalue)
  (`WidgetBlueprintLibrary.SetInputMode_UIOnlyEx` _returnvalue null)
  (`GameplayStatics.SetGamePaused` true)
  (switch `/Game/Data/Gameplay/E_Levels` (`/Game/Blueprints/Game/BP_GameInstance.SelectedLevel` (`self.As BP Game Instance`))
    (:`NewEnumerator1`
      _)
    (:`NewEnumerator2`
      _))
  (set `self.CurrentLevelData` (make `/Game/Blueprints/SaveGame/ST_LevelData` _currentleveldata_playtest _currentleveldata_hero _currentleveldata_level true _currentleveldata_timetaken _currentleveldata_enemieskilled))
  (message `/Game/Blueprints/SaveGame/BPI_SaveGame.SaveGame` (`self.As BP Game Instance`) (`self.CurrentLevelData`)))

(fn `OnPlayerDeathh`
  (bind _returnvalue (`GameplayStatics.GetPlayerController` 0))
  (bind (_currentleveldata_playtest _currentleveldata_hero _currentleveldata_level _currentleveldata_success _currentleveldata_timetaken _currentleveldata_enemieskilled) (break `/Game/Blueprints/SaveGame/ST_LevelData` (`self.CurrentLevelData`)))
  (bind _returnvalue_2 (`|CreateWidget` (`self.DeathScreenWidget`)))
  (`UserWidget.AddToViewport` _returnvalue_2 0)
  (set `PlayerController.bShowMouseCursor` true _returnvalue)
  (`WidgetBlueprintLibrary.SetInputMode_UIOnlyEx` _returnvalue _returnvalue_2)
  (`GameplayStatics.SetGamePaused` true)
  (set `self.CurrentLevelData` (make `/Game/Blueprints/SaveGame/ST_LevelData` _currentleveldata_playtest _currentleveldata_hero _currentleveldata_level false _currentleveldata_timetaken _currentleveldata_enemieskilled))
  (message `/Game/Blueprints/SaveGame/BPI_SaveGame.SaveGame` (`self.As BP Game Instance`) (`self.CurrentLevelData`)))

(fn `setAttackingState`
  (params (isAttacking :type Boolean))
  (bind (_herostate_inattackrange _herostate_istakingdamage _herostate_isinvulnerable _herostate_isattacking _herostate_isdashing _herostate_isjumping) (break `/Game/Data/Hero/ST_HeroState` (`self.HeroState`)))
  (set `self.HeroState` (make `/Game/Data/Hero/ST_HeroState` _herostate_inattackrange _herostate_istakingdamage _herostate_isinvulnerable isAttacking _herostate_isdashing _herostate_isjumping)))

(fn `setDashingState`
  (params (isDashing :type Boolean))
  (bind (_herostate_inattackrange _herostate_istakingdamage _herostate_isinvulnerable _herostate_isattacking _herostate_isdashing _herostate_isjumping) (break `/Game/Data/Hero/ST_HeroState` (`self.HeroState`)))
  (set `self.HeroState` (make `/Game/Data/Hero/ST_HeroState` _herostate_inattackrange _herostate_istakingdamage _herostate_isinvulnerable _herostate_isattacking isDashing _herostate_isjumping)))

(fn `setInvulnerableState`
  (params (isInvulnerable :type Boolean))
  (bind (_herostate_inattackrange _herostate_istakingdamage _herostate_isinvulnerable _herostate_isattacking _herostate_isdashing _herostate_isjumping) (break `/Game/Data/Hero/ST_HeroState` (`self.HeroState`)))
  (set `self.HeroState` (make `/Game/Data/Hero/ST_HeroState` _herostate_inattackrange _herostate_istakingdamage isInvulnerable _herostate_isattacking _herostate_isdashing _herostate_isjumping)))

(fn `setJumpingState`
  (params (isJumping :type Boolean))
  (bind (_herostate_inattackrange _herostate_istakingdamage _herostate_isinvulnerable _herostate_isattacking _herostate_isdashing) (break `/Game/Data/Hero/ST_HeroState` (`self.HeroState`)))
  (set `self.HeroState` (make `/Game/Data/Hero/ST_HeroState` _herostate_inattackrange _herostate_istakingdamage _herostate_isinvulnerable _herostate_isattacking _herostate_isdashing isJumping)))

(fn `setTakingDamageState`
  (params (isTakingDamage :type Boolean))
  (bind (_herostate_inattackrange _herostate_istakingdamage _herostate_isinvulnerable _herostate_isattacking _herostate_isdashing _herostate_isjumping) (break `/Game/Data/Hero/ST_HeroState` (`self.HeroState`)))
  (set `self.HeroState` (make `/Game/Data/Hero/ST_HeroState` _herostate_inattackrange isTakingDamage _herostate_isinvulnerable _herostate_isattacking _herostate_isdashing _herostate_isjumping)))

(fn `UpdateEnemyCount`
  (bind _outactors (`GameplayStatics.GetAllActorsOfClass` "/Game/Blueprints/Enemies/BP_Enemy.BP_Enemy_C"))
  (set `self.TotalEnemiesLeftInLevel` (`KismetArrayLibrary.Array_Length` _outactors)))

(fn `UserConstructionScript`)