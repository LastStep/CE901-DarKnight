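; BP_EnemyDrop is a pickup actor left by enemies that shows an item flipbook and expires after its lifespan.
; On begin play it assigns the configured flipbook to the Item component and starts the lifespan timer.
; When BP_Character overlaps its collision, it passes its ItemData to that character's item-drop event, then destroys itself after a zero-length delay.
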(event `self.ReceiveBeginPlay`
  (`PaperFlipbookComponent.SetFlipbook` (`self.Item`) (`|ConvertAsset` (`self.ItemFlipBook`)))
  (`self.SetLifeSpan` (`self.Lifespan`)))

(event `self.Collision.OnComponentBeginOverlap`
  (params (OverlappedComponent :type "PrimitiveComponent Object Reference") (OtherActor :type "Actor Object Reference") (OtherComp :type "PrimitiveComponent Object Reference") (OtherBodyIndex :type Integer) (bFromSweep :type Boolean) (SweepResult :type "HitResult Structure (by ref)"))
  (bind _asbp_character (cast `/Game/Blueprints/Heroes/PaperZD/BP_Character` OtherActor))
  (`/Game/Blueprints/Heroes/PaperZD/BP_Character.EventOnGettingItemDrop` _asbp_character (`self.ItemData`))
  (`KismetSystemLibrary.Delay` 0.0)
  (`self.K2_DestroyActor`))

(fn `UserConstructionScript`)