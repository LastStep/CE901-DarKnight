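; Behavior tree task that brings an enemy within attack range of the blackboard target character.
; Melee and ranged enemies use AI MoveTo toward the target, with the enemy data's attack range as acceptance radius, succeeding or failing with the move.
; Static enemies never move; the task only succeeds if the target is already within the blackboard attack range.
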(event `self.ReceiveExecuteAI`
  (params (OwnerController :type "AIController Object Reference") (ControlledPawn :type "Pawn Object Reference"))
  (bind _asbp_enemy (cast `/Game/Blueprints/Enemies/BP_Enemy` ControlledPawn))
  (bind _output_get (set `self.As BP Enemy` _asbp_enemy))
  (bind _asbp_character (cast `/Game/Blueprints/Heroes/PaperZD/BP_Character` (`BTFunctionLibrary.GetBlackboardValueAsActor` (`self.TargetActor`))))
  (set `self.As BP Character` _asbp_character)
  (switch `/Game/Data/Enemy/E_EnemyType` (`/Game/Data/Enemy/BP_EnemyDataAsset.EnemyType` (`/Game/Blueprints/Enemies/BP_Enemy.EnemyData` _output_get))
    (:`NewEnumerator0`
      (`|AIMoveTo` (`self.As BP Enemy`) (`CharacterMovementComponent.GetLastUpdateLocation` (`Character.CharacterMovement` (`self.As BP Character`))) (`self.As BP Character`) (`/Game/Data/Enemy/BP_EnemyDataAsset.AttackRange` (`/Game/Blueprints/Enemies/BP_Enemy.EnemyData` (`self.As BP Enemy`))) true :!label _label
        (:`OnSuccess`
          (`self.FinishExecute` true))
        (:`OnFail`
          (`self.FinishExecute` false))))
    (:`NewEnumerator1`
      (goto _label))
    (:`NewEnumerator3`
      ;[1 1 1] Not moving further if static enemies are out of range
      (if (>= (`BTFunctionLibrary.GetBlackboardValueAsFloat` (`self.AttackRange`)) (`KismetMathLibrary.Vector_Distance` (`Actor.K2_GetActorLocation` (`self.As BP Character`)) (`Actor.K2_GetActorLocation` (`self.As BP Enemy`))))
        (`self.FinishExecute` true)
        (else
          (`self.FinishExecute` false))))))