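; Base AI controller for BP_Enemy pawns that runs their behavior tree against the player character.
; BeginPlay initializes the BB_AIBoard blackboard.
; On possessing a BP_Enemy, it waits briefly, starts the tree, then seeds blackboard keys for the target, attack radius, defend radius and attack cooldown.
; Attack range and charge time come from the enemy's EnemyData, while the target is player 0 and the defend radius is hardcoded.
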(event `self.ReceiveBeginPlay`
  (bind _blackboardcomponent (`self.UseBlackboard` "/Game/Blueprints/AI/BB_AIBoard.BB_AIBoard"))
  (set `self.AI Blackboard` _blackboardcomponent))

(event `self.ReceivePossess`
  (params (PossessedPawn :type "Pawn Object Reference"))
  (bind _asbp_enemy (cast `/Game/Blueprints/Enemies/BP_Enemy` PossessedPawn))
  (set `self.Possessed Pawn` _asbp_enemy)
  (`KismetSystemLibrary.Delay` 0.2)
  (`self.RunBehaviorTree` (`self.AI Tree`))
  (`BlackboardComponent.SetValueAsObject` (`self.Blackboard`) (`self.TargetActorKeyName`) (`GameplayStatics.GetPlayerCharacter` 0))
  (`BlackboardComponent.SetValueAsFloat` (`self.Blackboard`) (`self.AttackRadiusKeyName`) (`/Game/Data/Enemy/BP_EnemyDataAsset.AttackRange` (`/Game/Blueprints/Enemies/BP_Enemy.EnemyData` (`self.Possessed Pawn`))))
  (`BlackboardComponent.SetValueAsFloat` (`self.Blackboard`) (`self.DefendRadiusKeyName`) 100.0)
  (`BlackboardComponent.SetValueAsFloat` (`self.Blackboard`) (`self.AttackCooldownKeyName`) (`/Game/Data/Enemy/BP_EnemyDataAsset.AttackChargeTime` (`/Game/Blueprints/Enemies/BP_Enemy.EnemyData` (`self.Possessed Pawn`)))))

(fn `UserConstructionScript`)