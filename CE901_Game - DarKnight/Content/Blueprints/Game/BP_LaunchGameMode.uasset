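; Launch game mode that runs the front-end menu flow and opens the chosen level.
; On BeginPlay it applies user settings, shows the main menu and switches to UI-only input with a mouse cursor.
; Selection events swap widgets from main menu to player select to level select.
; StartGame restores game-only input, then opens the level matching the SelectedLevel stored in BP_GameInstance.
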(event `self.ReceiveBeginPlay`
  (bind _returnvalue (`GameplayStatics.GetPlayerController` 0))
  (bind _returnvalue_2 (`GameUserSettings.GetGameUserSettings`))
  (`GameUserSettings.ApplySettings` _returnvalue_2 false)
  (bind _returnvalue_3 (`|CreateWidget` (`self.WB_MainMenu`)))
  (bind _output_get (set `self.MainMenuWidget` _returnvalue_3))
  (`UserWidget.AddToViewport` _output_get 0)
  (set `PlayerController.bShowMouseCursor` true _returnvalue)
  (`WidgetBlueprintLibrary.SetInputMode_UIOnlyEx` _returnvalue null))

(event `EventOnSelectingPlayTest`
  (`Widget.RemoveFromParent` (`self.MainMenuWidget`))
  (bind _returnvalue (`|CreateWidget` (`self.WB_PlayerSelect`)))
  (bind _output_get (set `self.PlayerSelectWidget` _returnvalue))
  (`UserWidget.AddToViewport` _output_get 0))

(event `EventOnSelectingHero`
  (`Widget.RemoveFromParent` (`self.PlayerSelectWidget`))
  (bind _returnvalue (`|CreateWidget` (`self.WB_LevelSelect`)))
  (bind _output_get (set `self.LevelSelectWidget` _returnvalue))
  (`UserWidget.AddToViewport` _output_get 0))

(fn `StartGame`
  (bind _returnvalue (`GameplayStatics.GetPlayerController` 0))
  (set `PlayerController.bShowMouseCursor` false _returnvalue)
  (`WidgetBlueprintLibrary.SetInputMode_GameOnly` _returnvalue)
  (bind _asbp_game_instance (cast `/Game/Blueprints/Game/BP_GameInstance` (`GameplayStatics.GetGameInstance`)))
  (switch `/Game/Data/Gameplay/E_Levels` (`/Game/Blueprints/Game/BP_GameInstance.SelectedLevel` _asbp_game_instance)
    (:`NewEnumerator0`
      (`GameplayStatics.OpenLevelBySoftObjectPtr` "/Game/Maps/Tutorial/Tutorial.Tutorial"))
    (:`NewEnumerator1`
      (`GameplayStatics.OpenLevelBySoftObjectPtr` "/Game/Maps/CityHouse/Basic.Basic"))
    (:`NewEnumerator2`
      (`GameplayStatics.OpenLevelBySoftObjectPtr` "/Game/Maps/CityRise/CityRiseLevel.CityRiseLevel"))))

(fn `UserConstructionScript`)