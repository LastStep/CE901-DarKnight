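; Base ability actor for hero attacks and passives, with a box hitbox sized and offset at construction.
; Activation sets the game mode's attacking state, then switches on ability type and hero class, casting self to the matching child class to call its Activate.
; Dash selection is an empty stub.
; ApplyDamage gathers enemies overlapping the hitbox and passes itself to each one's OnTakingDamage, exposing Power as damage.
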(event `self.ReceiveBeginPlay`
  (`self.SetReferences`))

(event `ActivateAbility`
  (`/Game/Blueprints/Game/BP_PlayGameMode.setAttackingState` (`self.CurrentGameMode`) true)
  (switch `/Game/Data/Gameplay/E_GameplayAbilityType` (`self.AbilityType`)
    (:`NewEnumerator3`
      (`self.SelectPassiveAbility`))
    (:`NewEnumerator4`
      (`self.SelectDash`))
    (:`NewEnumerator0`
      (`self.SelectLightAbility`))
    (:`NewEnumerator1`
      (`self.SelectHeavyAbility`))
    (:`NewEnumerator2`
      (`self.SelectLightChargedAbility`))))

(event `DeactivateAbility`
  (`/Game/Blueprints/Game/BP_PlayGameMode.setAttackingState` (`self.CurrentGameMode`) false))

(fn `ApplyDamage`
  (for _array_element (`self.GetEnemiesHit`)
    (`/Game/Blueprints/Interface/BPI_Hit.onTakingDamage` _array_element _array_element self)))

(fn `GetDamageFromAbility`
  (returns (Damage :type "Float (double-precision)"))
  (return (`self.Power`)))

(fn `GetEnemiesHit`
  (returns (`Enemies Hit` :type "Array of /Game/Blueprints/Enemies/BP_Enemy Object Reference"))
  (locals (EnemiesHit :type "Array of /Game/Blueprints/Enemies/BP_Enemy Object Reference"))
  (for _array_element (`PrimitiveComponent.GetOverlappingActors` (`self.AbilityHitbox`) "/Game/Blueprints/Enemies/BP_Enemy.BP_Enemy_C")
    (bind _asbp_enemy (cast `/Game/Blueprints/Enemies/BP_Enemy` _array_element))
    (`KismetArrayLibrary.Array_Add` (`local.EnemiesHit`) _asbp_enemy))
  (return (`local.EnemiesHit`)))

(fn `SetAbilityHitbox`
  (params (OffsetX :type Integer) (OffsetZ :type Integer) (Length :type Integer) (Height :type Integer))
  (bind _abilityhitbox (`self.AbilityHitbox`))
  (`BoxComponent.SetBoxExtent` _abilityhitbox (`KismetMathLibrary.MakeVector` (`KismetMathLibrary.Conv_IntToDouble` Length) 50.0 (`KismetMathLibrary.Conv_IntToDouble` Height)) true)
  (`SceneComponent.K2_AddLocalOffset` _abilityhitbox (`KismetMathLibrary.MakeVector` (+ (/ Length 2) OffsetX) 0.0 (+ (/ Height 2) OffsetZ)) false false))

(fn `SetReferences`
  (bind _asbp_character (cast `/Game/Blueprints/Heroes/PaperZD/BP_Character` (`GameplayStatics.GetPlayerCharacter` 0)))
  (bind _output_get (set `self.Hero` _asbp_character))
  (bind _asabp_hero_core (cast `/Game/Blueprints/Heroes/ABP_hero_core` (`PaperZDCharacter.AnimInstance` _output_get)))
  (set `self.HeroAnimInstance` _asabp_hero_core)
  (bind _asbp_play_game_mode (cast `/Game/Blueprints/Game/BP_PlayGameMode` (`GameplayStatics.GetGameMode`)))
  (set `self.CurrentGameMode` _asbp_play_game_mode))

(fn `UserConstructionScript`
  (`self.SetAbilityHitbox` (`self.HitboxOffsetX`) (`self.HitboxOffsetZ`) (`self.HitboxLength`) (`self.HitboxHeight`)))