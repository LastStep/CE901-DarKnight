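; Demo player controller for side-on character movement along world X, with a pause toggle.
; Adds the Enhanced Input mapping context on BeginPlay and caches the character and game mode.
; Forward input, ignored while the game mode's hero state is attacking, sets control yaw to face left or right and adds movement.
; Pause input toggles the pause menu, cursor and game pause, notifying BP_Character of each change.
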(event `self.ReceiveBeginPlay`
  (bind _asbp_character (cast `/Game/Blueprints/Heroes/PaperZD/BP_Character` (`GameplayStatics.GetPlayerCharacter` 0)))
  (set `self.As BP Character` _asbp_character)
  (bind _asbp_play_game_mode (cast `/Game/Blueprints/Game/BP_PlayGameMode` (`GameplayStatics.GetGameMode`)))
  (set `self.CurrentGameMode` _asbp_play_game_mode)
  (`EnhancedInputSubsystemInterface.AddMappingContext` (pcsubsystem `EnhancedInputLocalPlayerSubsystem` self) "/Game/Actions/IMC_PlayerControls.IMC_PlayerControls" 1 (struct)))

(event `EnhancedInput|/Game/Actions/Inputs/CharacterInputs/IA_Forward`
  (params (ActionValue :type "Float (double-precision)") (ElapsedSeconds :type "Float (double-precision)") (TriggeredSeconds :type "Float (double-precision)") (InputAction :type "InputAction Object Reference" :default "/Game/Actions/Inputs/CharacterInputs/IA_Forward.IA_Forward"))
  (bind (_herostate_inattackrange _herostate_istakingdamage _herostate_isinvulnerable _herostate_isattacking) (break `/Game/Data/Hero/ST_HeroState` (`/Game/Blueprints/Game/BP_PlayGameMode.HeroState` (`self.CurrentGameMode`))))
  (:`Triggered`
    (if (not _herostate_isattacking)
      (set `self.Axis Value` ActionValue)
      (`self.MoveForward`))))

(event `EnhancedInput|/Game/Actions/Inputs/GameInputs/IA_Pause`
  (params (ActionValue :type Boolean) (ElapsedSeconds :type "Float (double-precision)") (TriggeredSeconds :type "Float (double-precision)") (InputAction :type "InputAction Object Reference" :default "/Game/Actions/Inputs/GameInputs/IA_Pause.IA_Pause"))
  (:`Started`
    (`self.OnPressingPause`)))

(fn `MoveForward`
  (bind _returnvalue (`GameplayStatics.GetPlayerPawn` 0))
  (bind _axis_value (`self.Axis Value`))
  (bind _returnvalue_2 (`Pawn.GetController` _returnvalue))
  (`/Engine/EditorBlueprintResources/StandardMacros.CompareFloat` _axis_value
    (:`>`
      ;[0 0.4745 1] Look Right
      (`/Engine/EditorBlueprintResources/StandardMacros.IsValid` _returnvalue_2
        (:`Is Valid`
          (`self.SetControlRotation` _returnvalue_2 (`KismetMathLibrary.MakeRotator` 0.0)))))
    (:`<`
      ;[0 0.4745 1] Look Left
      (`/Engine/EditorBlueprintResources/StandardMacros.IsValid` _returnvalue_2
        (:`Is Valid`
          (`self.SetControlRotation` _returnvalue_2 (`KismetMathLibrary.RInterpTo` (`self.GetControlRotation`) (`KismetMathLibrary.MakeRotator` 0.0 0.0 180.0) (`GameplayStatics.GetWorldDeltaSeconds`)))))))
  (`Pawn.AddMovementInput` _returnvalue (1.0 0.0 0.0) _axis_value false))

(fn `OnPressingPause`
  (if (`GameplayStatics.IsGamePaused`)
    (`self.ResumeGame`)
    (else
      (`self.PauseGame`))))

(fn `PauseGame`
  (bind _returnvalue (`|CreateWidget` "/Game/Blueprints/UI/WB_PauseMenu.WB_PauseMenu_C" self))
  (bind _output_get (set `self.PauseMenuWdiget` _returnvalue))
  (`UserWidget.AddToViewport` _output_get 0)
  (`WidgetBlueprintLibrary.SetInputMode_GameAndUIEx` self (`self.PauseMenuWdiget`))
  (set `self.bShowMouseCursor` true)
  (`GameplayStatics.SetGamePaused` true)
  (bind _asbp_character (cast `/Game/Blueprints/Heroes/PaperZD/BP_Character` (`GameplayStatics.GetPlayerPawn` 0)))
  (`/Game/Blueprints/Heroes/PaperZD/BP_Character.OnGamePause` _asbp_character))

(fn `ResumeGame`
  (`Widget.RemoveFromParent` (`self.PauseMenuWdiget`))
  (`WidgetBlueprintLibrary.SetInputMode_GameAndUIEx` self null)
  (set `self.bShowMouseCursor` false)
  (`GameplayStatics.SetGamePaused` false)
  (bind _asbp_character (cast `/Game/Blueprints/Heroes/PaperZD/BP_Character` (`GameplayStatics.GetPlayerPawn` 0)))
  (`/Game/Blueprints/Heroes/PaperZD/BP_Character.OnGameResume` _asbp_character))

(fn `UserConstructionScript`)